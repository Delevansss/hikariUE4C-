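; Eagle rotation puzzle actor that the player aligns to a stored solution rotation to unlock a linked puzzle actor.
; Use requires a placed tablet, then either reports collected fragments or, once all are found, starts fixed-camera inspection with the player hidden.
; Look axes rotate the pivot while a looping timer checks it against per-axis tolerances.
; Success or menu exit restores the player view and eases rotation to solved or starting values via timeline.
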(event `CE_多次点击`
  (bind `_此关卡开启解谜的碎片数量` (`self.此关卡开启解谜的碎片数量`))
  (bind _collected_puzzle_nums (`self.Collected Puzzle Nums`))
  (goto _label :!via `Reset`))

(event `self.ReceiveTick`
  (params (DeltaSeconds :type "Float (single-precision)"))
  (bind `_此关卡开启解谜的碎片数量` (`self.此关卡开启解谜的碎片数量`))
  (bind _collected_puzzle_nums (`self.Collected Puzzle Nums`))
  (bind _collected_puzzle_nums_2 (`self.Collected Puzzle Nums`))
  (`|ExecutionSequence`
    (:`then_0`
      (set `self.Collected Puzzle Nums` _collected_puzzle_nums)
      (if (`self.Det`)
        (if (== _collected_puzzle_nums (`self.此关卡开启解谜的碎片数量`))
          (`|ExecutionSequence`
            (:`then_0`
              (`/Engine/EditorBlueprintResources/StandardMacros.DoOnce` false
                (:`Completed`
                  (`/Game/HorrorEngine/Blueprints/Core/HorrorEngineFunctions.Notice` "" "可以" "解谜")
                  (`SceneComponent.SetVisibility` (`self.StaticMesh`) true false)))))
          (else
            (`/Engine/EditorBlueprintResources/StandardMacros.DoOnce` false :!label _label
              (:`Completed`
                (`TextBlock.SetText` (`/Game/EaglePuzzle/Puzzle_UMG.剩余碎片` (`self.PuzzleUMG`)) (`KismetTextLibrary.Conv_IntToText` (- `_此关卡开启解谜的碎片数量` _collected_puzzle_nums_2)))
                (`/Game/HorrorEngine/Blueprints/Core/HorrorEngineFunctions.Notice` "碎片数量:" (`KismetTextLibrary.Conv_IntToText` _collected_puzzle_nums_2) (`|FormatText` "/{iit}" `_此关卡开启解谜的碎片数量`))
                (`SceneComponent.SetVisibility` (`self.StaticMesh`) false false)))))))
    (:`then_1`
      (if (`self.IsInspecting`)
        (set `/Game/EaglePuzzle/PuzzleActor.CanBeUsed` true (`self.绑定puzzleactor`))
        (`PlayerController.SetViewTargetWithBlend` (`GameplayStatics.GetPlayerController` 0) (`self.固定视角镜头`) 1.0 "VTBlend_Linear" 0.0 true)
        (`SceneComponent.SetHiddenInGame` (`Character.Mesh` (`GameplayStatics.GetPlayerCharacter` 0)) true false)))))

(event `self.ReceiveBeginPlay`
  (bind _staticmesh (`self.StaticMesh`))
  (bind _returnvalue (`|CreateWidget` "/Game/EaglePuzzle/Puzzle_UMG.Puzzle_UMG_C" (`GameplayStatics.GetPlayerController` 0)))
  (bind _output_get (set `self.PuzzleUMG` _returnvalue))
  (`UserWidget.AddToViewport` _output_get 0)
  (`self.DisableInput` (`GameplayStatics.GetPlayerController` 0))
  (if (== (`self.此关卡开启解谜的碎片数量`) 0)
    (`SceneComponent.SetVisibility` _staticmesh true false)
    (else
      (`SceneComponent.SetVisibility` _staticmesh false false))))

(event `提取旋转物体正确值`
  (bind _output_get (set `self.PuzzleSovledRotation` (`SceneComponent.K2_GetComponentRotation` (`self.Pivot`))))
  (`KismetSystemLibrary.PrintString` (`KismetStringLibrary.Concat_StrStr` "提取旋转物体正确值" (`KismetStringLibrary.Conv_RotatorToString` _output_get))))

(event `重置到正确值`
  (`KismetSystemLibrary.PrintString` "重置到正确值")
  (`self.K2_SetActorRotation` (`self.PuzzleSovledRotation`)))

(event `开始旋转`
  (set `self.StartRotation` (`SceneComponent.K2_GetComponentRotation` (`self.Pivot`))))

(event `self.Use`
  (params (HorrorEvent :type Boolean))
  (if (and (`/Game/HorrorEngine/Blueprints/UsableAssets/Electronics/TabletLoat.LoatHasTalet` (`self.TabletLoat`)) (not (`self.PuzzleSovled`)))
    (`|ExecutionSequence`
      (:`then_0`
        (set `self.Det` true)
        (if (== (`self.Collected Puzzle Nums`) (`self.此关卡开启解谜的碎片数量`))
          (set `self.IsInspecting` true)
          (set `self.CanRotate` false)
          (`/Game/HorrorEngine/Blueprints/Core/HorrorEngineFunctions.PlayerInput` false)
          (`self.EnableInput` (`GameplayStatics.GetPlayerController` 0))
          (`MovementComponent.StopMovementImmediately` (`Character.CharacterMovement` (`GameplayStatics.GetPlayerCharacter` 0)))
          (else
            (`self.CE_多次点击`))))
      (:`then_1`
        (`self.EventCheckPuzzle` true)))
    (else
      (`/Game/HorrorEngine/Blueprints/Core/HorrorEngineFunctions.Notice` "请" "放置手机到到合适位置。" "！！"))))

(event `InputAxis|[HE]Turn`
  (params (AxisValue :type "Float (single-precision)"))
  ;[0.498 0.6737 1] Look Settings
  (`SceneComponent.K2_AddWorldRotation` (`self.Pivot`) (* (`KismetMathLibrary.MakeRotator` 0.0 0.0 (* AxisValue 0.1)) (`self.RotationSpeed`)) false false))

(event `EventCheckPuzzle`
  (params (Start :type Boolean))
  (if Start
    (`KismetSystemLibrary.K2_SetTimer` null "CheckPuzzle" 0.1 true)
    (else
      (`KismetSystemLibrary.K2_SetTimer` null "CheckPuzzle" 0.0 true))))

(event `InputAxis|[HE]LookUp`
  (params (AxisValue :type "Float (single-precision)"))
  ;[0.498 0.6737 1] Look Settings
  (`SceneComponent.K2_AddWorldRotation` (`self.Pivot`) (* (`KismetMathLibrary.MakeRotator` 0.0 (* AxisValue -0.1)) (`self.RotationSpeed`)) false false))

(event `InputAction|[HE]Menu`
  (params (Key :type "Key Structure"))
  ;[0.498 0.6737 1] Look Settings
  (:`Pressed`
    (`self.PuzzleSovling`)))

(event `PuzzleSovling`
  (`PlayerController.SetViewTargetWithBlend` (`GameplayStatics.GetPlayerController` 0) (`GameplayStatics.GetPlayerCharacter` 0) 1.0 "VTBlend_Linear" 0.0 true)
  (`|ExecutionSequence`
    (:`then_0`
      (`KismetSystemLibrary.Delay` 1.0)
      (bind _asmaster (`/Game/HorrorEngine/Blueprints/Core/HorrorEngineFunctions.GetPlayer`))
      (`self.EnableInput` _asmaster (`GameplayStatics.GetPlayerController` 0)))
    (:`then_1`
      (`SceneComponent.SetHiddenInGame` (`Character.Mesh` (`GameplayStatics.GetPlayerCharacter` 0)) false false)
      (bind (_direction _smooth) (`Timeline|Sovling` :!via `PlayFromStart`)
        (:`Update`
          (`self.K2_SetActorRotation` (`KismetMathLibrary.RLerp` (`self.K2_GetActorRotation`) (`KismetMathLibrary.SelectRotator` (`self.PuzzleSovledRotation`) (`self.StartRotation`) (`self.PuzzleSovled`)) _smooth true)))
        (:`Finished`
          (`self.DisableInput` (`GameplayStatics.GetPlayerController` 0))
          (`/Game/HorrorEngine/Blueprints/Core/HorrorEngineFunctions.PlayerInput` true)
          (`SceneComponent.SetHiddenInGame` (`Character.Mesh` (`GameplayStatics.GetPlayerCharacter` 0)) false false)
          (if (`self.PuzzleSovled`)
            (`self.Unlock` (`self.绑定puzzleactor`) false)))))))

(event `PickUpp`)

(fn `CheckPuzzle`
  (bind (`_修正阈值_roll` `_修正阈值_pitch` `_修正阈值_yaw`) (`KismetMathLibrary.BreakRotator` (`self.修正阈值`)))
  (bind (_puzzlesovledrotation_roll _puzzlesovledrotation_pitch _puzzlesovledrotation_yaw) (`KismetMathLibrary.BreakRotator` (`self.PuzzleSovledRotation`)))
  (bind `_修正阈值_roll_2` (`KismetMathLibrary.BreakRotator` (`self.修正阈值`)))
  (bind _puzzlesovledrotation_roll_2 (`KismetMathLibrary.BreakRotator` (`self.PuzzleSovledRotation`)))
  (bind (`_修正阈值_roll_3` `_修正阈值_pitch_2`) (`KismetMathLibrary.BreakRotator` (`self.修正阈值`)))
  (bind (_puzzlesovledrotation_roll_3 _puzzlesovledrotation_pitch_2) (`KismetMathLibrary.BreakRotator` (`self.PuzzleSovledRotation`)))
  (`KismetSystemLibrary.PrintString` "开始Check" true true (struct :`R` 1.0 :`B` 0.385657 :`A` 1.0) 0.0)
  (if (`self.IsInspecting`)
    (if (and (`KismetMathLibrary.InRange_FloatFloat` (.roll (`SceneComponent.K2_GetComponentRotation` (`self.Pivot`))) (- _puzzlesovledrotation_roll_2 `_修正阈值_roll_2`) (+ _puzzlesovledrotation_roll_2 `_修正阈值_roll_2`)) (`KismetMathLibrary.InRange_FloatFloat` (.pitch (`SceneComponent.K2_GetComponentRotation` (`self.Pivot`))) (- _puzzlesovledrotation_pitch_2 `_修正阈值_pitch_2`) (+ _puzzlesovledrotation_pitch_2 `_修正阈值_pitch_2`)) (`KismetMathLibrary.InRange_FloatFloat` (.yaw (`SceneComponent.K2_GetComponentRotation` (`self.Pivot`))) (- _puzzlesovledrotation_yaw `_修正阈值_yaw`) (+ _puzzlesovledrotation_yaw `_修正阈值_yaw`)))
      (set `self.PuzzleSovled` true)
      (`self.PuzzleSovling`)
      (set `self.StartRotation` (`KismetMathLibrary.ComposeRotators` (`self.修正阈值`) (`self.StartRotation`)))
      (set `self.IsInspecting` false)
      (`MovementComponent.StopMovementImmediately` (`Character.CharacterMovement` (`GameplayStatics.GetPlayerCharacter` 0)))
      (else
        (set `self.PuzzleSovled` false)))))

(fn `UserConstructionScript`
  (`StaticMeshComponent.SetStaticMesh` (`self.StaticMesh`) (`self.Puzzle Mesh`))
  (`/Game/HorrorEngine/Blueprints/Core/HorrorEngineMacros.HM_DefaultConstructions` (`self.CreateNewHorrorEvent`)))